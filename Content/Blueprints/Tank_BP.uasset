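; Player-controlled tank Blueprint that simulates physics and routes input to movement, camera aiming and firing.
; On begin play it hands both tracks to TankMovement, with left and right swapped, and registers the barrel and turret.
; Throttle axes drive each track directly, while forward and turn axes go through TankMovement intents.
; Aim axes rotate the azimuth gimbal and spring arm, scaled by delta time, and the Fire action calls Fire.
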(event `self.ReceiveBeginPlay`
  (`PrimitiveComponent.SetSimulatePhysics` (`self.Tank`) true)
  (`TankMovementComponent.Initialise` (`self.TankMovement`) (`self.RightTrack`) (`self.LeftTrack`))
  (`self.SetBarrelReference` (`self.Barrel`))
  (`self.SetTurretReference` (`self.Turret`)))

(event `InputAxis|LeftThrottle`
  (params (AxisValue :type "Float (single-precision)"))
  ;[1 1 1] Movement
  (`TankTrack.SetThrottle` (`self.LeftTrack`) AxisValue))

(event `InputAxis|TurnRight`
  (params (AxisValue :type "Float (single-precision)"))
  ;[1 1 1] Movement
  (`/Engine/EditorBlueprintResources/StandardMacros.NegateFloat` AxisValue
    (:`  `
      (`TankMovementComponent.IntendTurnRight` (`self.TankMovement`) AxisValue))))

(event `InputAxis|RightThrottle`
  (params (AxisValue :type "Float (single-precision)"))
  ;[1 1 1] Movement
  (`TankTrack.SetThrottle` (`self.RightTrack`) AxisValue))

(event `InputAxis|MoveForward`
  (params (AxisValue :type "Float (single-precision)"))
  ;[1 1 1] Movement
  (`TankMovementComponent.IntendMoveForward` (`self.TankMovement`) AxisValue))

(event `InputAxis|AimAzimuth`
  (params (AxisValue :type "Float (single-precision)"))
  ;[1 1 1] Camera input binding
  (`SceneComponent.K2_AddLocalRotation` (`self.Azimuth_Gimbal`) (`KismetMathLibrary.MakeRotator` 0.0 0.0 (* AxisValue (`GameplayStatics.GetWorldDeltaSeconds`) 100.0)) false false))

(event `InputAxis|AImElevation`
  (params (AxisValue :type "Float (single-precision)"))
  ;[1 1 1] Camera input binding
  (`SceneComponent.K2_AddLocalRotation` (`self.SpringArm`) (`KismetMathLibrary.MakeRotator` 0.0 (* AxisValue (`GameplayStatics.GetWorldDeltaSeconds`) 100.0)) false false))

(event `InputAction|Fire`
  (params (Key :type "Key Structure" :default "AnyKey"))
  ;[1 1 1] Camera input binding
  (:`Pressed`
    (`self.Fire`)))

(fn `UserConstructionScript`)